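; Enemy AI character for a stealth game that patrols either random reachable points or randomly picked target points, and chases the player on sight.
; Tick chooses patrol or chase from CanMove and a visibility flag that PawnSensing sets and a short retriggerable delay clears.
; AIMoveTo drives movement at walk or run speed.
; Reaching the player widens sight radius, reaching target points shrinks it to a floor, and hearing only prints debug text.
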(event OnSeePawn(PawnSensing)
  (params (Pawn :type Pawn%20Object%20Reference))
  (Utilities|Casting|CastToBP_ThirdPersonCharacterCustom Pawn
    (:then
      (Utilities|FlowControl|Sequence
        (:then_0
          (Development|PrintString "Hey stop right there!" true true "(R=0.182292,G=0.000000,B=0.003534,A=1.000000)")
          (Variables|Default|SetbPlayerVisable true))
        (:then_1
          (Utilities|FlowControl|RetriggerableDelay 0.2)
          (Variables|Default|SetbPlayerVisable false))))
    (:CastFailed
      (Utilities|Casting|CastToBP_EnemyAI Pawn)
      (Development|PrintString "Hello there"))))

(event OnHearNoise(PawnSensing)
  (params (Instigator :type Pawn%20Object%20Reference) (Location :type Vector%20%28by%20ref%29 :default "0, 0, 0") (Volume :type Float%20%28single-precision%29))
  (Utilities|Casting|CastToBP_ThirdPersonCharacterCustom Instigator
    (:then
      (Development|PrintString "Heard a noise"))
    (:CastFailed
      (Development|PrintString "fadsfdsafdsafdsa"))))

(event Custom|ChasePlayer
  (bind _pawnsensing (Variables|Default|GetPawnSensing))
  (bind _sightradius (Variables|/Script/AIModule.PawnSensingComponent|GetSightRadius _pawnsensing))
  (if (Variables|Default|GetbPlayerVisable)
    (CallFunction|UpdateWalkSpeed 6e+02)
    (Variables|Default|SetcanMove false)
    (AI|AIMoveTo self "0, 0, 0" (Game|GetPlayerCharacter 0) 75.0 false
      (:OnSuccess
        (Development|PrintString "Bokn")
        (Variables|Default|SetcanMove true)
        (CallFunction|UpdateSightRadius (+ _sightradius 5.0))
        (Development|PrintText (Utilities|Text|ToText(Float) _sightradius "HalfToEven"))))))

(event Custom|PatrolRandom
  (CallFunction|UpdateWalkSpeed 2e+02)
  (Variables|Default|SetcanMove false)
  (AI|AIMoveTo self (.RandomLocation (AI|Navigation|GetRandomReachablePointinRadius (Transformation|GetActorLocation) (Variables|Default|GetRadiusPatrol) 0 0)) 0 75.0 false
    (:OnSuccess
      (Utilities|FlowControl|Delay (Math|Random|RandomFloatinRange 2.0 8.0))
      (Variables|Default|SetcanMove true))))

(event Custom|MoveToNextPatrolPoint
  (CallFunction|UpdateWalkSpeed 2e+02)
  (Variables|Default|SetcanMove false)
  (AI|AIMoveTo self "0, 0, 0" (Utilities|Array|Get(acopy) (Variables|Default|GetPatrolTargetPoints) (Variables|Default|GetpatrolTargetPointIndex)) 75.0 false
    (:OnSuccess
      (CallFunction|SetNextPatrolPointIndex)
      (Utilities|FlowControl|Delay (Math|Random|RandomFloatinRange 3.0 6.0))
      (Variables|Default|SetcanMove true)
      (CallFunction|UpdateSightRadius (- (Variables|/Script/AIModule.PawnSensingComponent|GetSightRadius (Variables|Default|GetPawnSensing)) 5.0))
      (if (< (Variables|/Script/AIModule.PawnSensingComponent|GetSightRadius (Variables|Default|GetPawnSensing)) 8e+02)
        (Variables|/Script/AIModule.PawnSensingComponent|SetSightRadius (Variables|Default|GetPawnSensing) 8e+02)))))

(event Custom|SetNextPatrolPointIndex
  (Variables|Default|SetpatrolTargetPointIndex (Math|Random|RandomIntegerinRange 0 (Utilities|Array|Length (Variables|Default|GetPatrolTargetPoints)))))

(event EventTick
  (params (DeltaSeconds :type Float%20%28single-precision%29))
  (if (Variables|Default|GetcanMove)
    (if (Variables|Default|GetbPlayerVisable)
      (CallFunction|ChasePlayer)
      (elif (Variables|Default|GettargetPointMovement)
        (CallFunction|MovetoNextPatrolPoint)
        (else
          (CallFunction|PatrolRandom))))
    (elif (Variables|Default|GetbPlayerVisable)
      (CallFunction|ChasePlayer))))

(fn ConstructionScript)

(fn UpdateWalkSpeed
  (params (newWalkSpeed :type Float%20%28double-precision%29))
  (Variables|/Script/Engine.CharacterMovementComponent|SetMaxWalkSpeed (Variables|Character|GetCharacterMovement) newWalkSpeed))

(fn UpdateSightRadius
  (params (Sight :type Float%20%28double-precision%29))
  (Variables|/Script/AIModule.PawnSensingComponent|SetSightRadius (Variables|Default|GetPawnSensing) Sight))