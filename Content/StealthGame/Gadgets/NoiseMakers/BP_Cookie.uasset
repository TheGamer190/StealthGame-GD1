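; BP_Cookie is a stealth-game pickup, commented as a rock, that the player can grab and carry in the right hand.
; Overlapping its sphere while it is unheld asks the custom player character to pick it up.
; Its Pickup event snaps the sphere to the hand_r socket and disables physics and collision.
; Pickup also changes the game mode's music, sets HasCookie on the player and starts the UI timer.
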(event OnComponentBeginOverlap(Sphere)
  (params (OverlappedComponent :type Primitive%20Component%20Object%20Reference) (OtherActor :type Actor%20Object%20Reference) (OtherComp :type Primitive%20Component%20Object%20Reference) (OtherBodyIndex :type Integer) (bFromSweep :type Boolean) (SweepResult :type Hit%20Result%20Structure%20%28by%20ref%29))
  ;[1 0.5395 0.008568] Pickup Rock
  (if (not (Variables|Default|GetbPickedUp)) ; If a rock is already picked up, ignore this overlap.
    (bind _asbp_third_person_character_custom (Utilities|Casting|CastToBP_ThirdPersonCharacterCustom OtherActor)) ; Make sure the overlapping actor is the player
    (Default|TrytoPickUp _asbp_third_person_character_custom self) ; Call TryToPickUp Event from BP_ThirdPersonCharacterCustom
  ))

(event EventPickup
  (params (ParentMesh :type Skeletal%20Mesh%20Component%20Object%20Reference))
  ;[1 0.5395 0.008568] Pickup Rock
  (Variables|Default|SetbPickedUp true) ; Flag that the rock is now being held
  (Transformation|AttachComponentToComponent (Variables|Default|GetSphere) ParentMesh "hand_r" "SnapToTarget" "KeepRelative" "KeepRelative" true) ; Snap the rock to the player's righ hand
  (Physics|SetSimulatePhysics (Variables|Default|GetSphere) false) ; Stop physics while holding
  (Collision|SetCollisionEnabled (Variables|Default|GetSphere) "NoCollision") ; Don't collide with me while I am holding you.
  (Variables|Default|SetbPickedUp true)
  (bind _asbp_third_person_game_mode_custom (Utilities|Casting|CastToBP_ThirdPersonGameModeCustom (Game|GetGameMode)))
  (Default|ChangeMusic _asbp_third_person_game_mode_custom)
  (bind _asbp_third_person_character_custom (Utilities|Casting|CastToBP_ThirdPersonCharacterCustom (Game|GetPlayerCharacter 0)))
  (Variables|/Game/StealthGame/Core/Characters/PlayerCharacter/BP_ThirdPersonCharacterCustom.BP_ThirdPersonCharacterCustom_C|SethasCookie _asbp_third_person_character_custom true)
  (Default|StartTimer (Variables|/Game/StealthGame/Core/Characters/PlayerCharacter/BP_ThirdPersonCharacterCustom.BP_ThirdPersonCharacterCustom_C|GetplayerUI _asbp_third_person_character_custom)))

(fn ConstructionScript)